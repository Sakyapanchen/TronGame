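; BP_TronCycle is a player-controlled Tron-style cycle that turns left or right on input.
; Turn presses, overlaps and hits pass straight to TurnLeft, TurnRight, CycleOverlap and CycleHit, whose logic is defined outside this graph.
; When the player ID arrives, cycles that are not locally controlled destroy their Indicator component, so only the local player's cycle keeps it.
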(event `self.ReceiveBeginPlay`
  (`parent.ReceiveBeginPlay`))

(event `InputAction|TurnLeft`
  (params (Key :type "Key Structure"))
  (:`Pressed`
    (`self.TurnLeft`)))

(event `InputAction|TurnRight`
  (params (Key :type "Key Structure"))
  (:`Pressed`
    (`self.TurnRight`)))

(event `self.ReceiveActorBeginOverlap`
  (params (OtherActor :type "Actor Object Reference"))
  (`self.CycleOverlap` OtherActor))

(event `self.ReceiveHit`
  (params (MyComp :type "PrimitiveComponent Object Reference") (Other :type "Actor Object Reference") (OtherComp :type "PrimitiveComponent Object Reference") (bSelfMoved :type Boolean) (HitLocation :type "Vector Structure") (HitNormal :type "Vector Structure") (NormalImpulse :type "Vector Structure") (Hit :type "HitResult Structure (by ref)"))
  (`self.CycleHit` Other))

(event `self.OnPlayerIdRecieved`
  (params (playerId :type Integer))
  (if (not (`self.IsLocallyControlled`))
    (`self.RemoveIndicator`)))

(fn `RemoveIndicator`
  (bind _indicator (`self.Indicator`)
    (:`then`
      (`ActorComponent.K2_DestroyComponent` _indicator))
    (:`else`)))

(fn `UserConstructionScript`)