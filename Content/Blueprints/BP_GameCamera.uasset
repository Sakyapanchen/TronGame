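; Game camera actor that becomes the first player's view and fits its orthographic width to the viewport.
; On BeginPlay, skipped on dedicated servers, it sets itself as player controller 0's view target, then calls UpdateCamera.
; UpdateCamera multiplies the camera component's existing OrthoWidth by the viewport aspect ratio and a fixed factor, applied only once at startup.
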(event `self.ReceiveBeginPlay`
  (bind _returnvalue (`GameplayStatics.GetPlayerController` 0))
  (if (not (`KismetSystemLibrary.IsDedicatedServer`))
    (`|ExecutionSequence`
      (:`then_0`
        (`/Engine/EditorBlueprintResources/StandardMacros.IsValid` _returnvalue
          (:`Is Valid`
            (`PlayerController.SetViewTargetWithBlend` _returnvalue self 0.0 "VTBlend_Linear" 0.0 false))))
      (:`then_1`
        (`self.UpdateCamera`)))))

(fn `UpdateCamera`
  (bind (_x _y) (`KismetMathLibrary.BreakVector2D` (`WidgetLayoutLibrary.GetViewportSize`)))
  (set `CameraComponent.OrthoWidth` (* (/ _x _y) (`CameraComponent.OrthoWidth` (`self.CameraComponent`)) 0.6) (`self.CameraComponent`)))

(fn `UserConstructionScript`)