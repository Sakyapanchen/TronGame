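; Light trail segment actor for a Tron cycle, drawn as a colored procedural quad that stretches behind its owning BP_TronCycle.
; BeginPlay creates a zero-length, collision-enabled mesh section with a dynamic material, sized across local Y by the cycle's TrailThickness.
; While active, Tick moves the far edge along local X by the distance to the cycle's trail source point, so the segment stays straight.
; GetReferences caches the owning cycle.
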(event `self.ReceiveActorBeginOverlap`
  (params (OtherActor :type "Actor Object Reference")))

(event `self.ReceiveTick`
  (params (DeltaSeconds :type "Float (single-precision)"))
  (bind _trailcolor (`self.TrailColor`))
  (bind _returnvalue (* (0.0 1.0 0.0) (/ (`TronCycle.TrailThickness` (`self.OwnerCycle`)) 2.0)))
  (bind _returnvalue_2 (* (0.0 -1.0 0.0) (/ (`TronCycle.TrailThickness` (`self.OwnerCycle`)) 2.0)))
  (bind _returnvalue_3 (`KismetMathLibrary.MakeVector` (`KismetMathLibrary.VSize` (- (`TronCycle.GetTrailSourcePoint` (`self.OwnerCycle`)) (`self.K2_GetActorLocation`)))))
  (`parent.ReceiveTick` DeltaSeconds)
  (if (`self.bIsActive`)
    (set `self.NewVar_0` (`|MakeArray` (+ _returnvalue_3 _returnvalue_2) (+ _returnvalue_3 _returnvalue) _returnvalue _returnvalue_2))
    (`ProceduralMeshComponent.UpdateMeshSection_LinearColor` :`self` (`self.TronProceduralMesh`) :`Vertices` (`self.NewVar_0`) :`UV0` (`|MakeArray` (0.0 0.0) (1.0 0.0) (1.0 1.0) (0.0 1.0) :!type "Vector2D Structure") :`VertexColors` (`|MakeArray` _trailcolor _trailcolor _trailcolor _trailcolor))))

(event `self.ReceiveBeginPlay`
  (bind _trailcolor (`self.TrailColor`))
  (bind _returnvalue (* (0.0 1.0 0.0) (/ (`TronCycle.TrailThickness` (`self.OwnerCycle`)) 2.0)))
  (bind _returnvalue_2 (* (0.0 -1.0 0.0) (/ (`TronCycle.TrailThickness` (`self.OwnerCycle`)) 2.0)))
  (bind _array (`|MakeArray` _returnvalue_2 _returnvalue _returnvalue _returnvalue_2))
  (`parent.ReceiveBeginPlay`)
  (set `self.NewVar_0` _array)
  (`ProceduralMeshComponent.CreateMeshSection_LinearColor` :`self` (`self.TronProceduralMesh`) :`Vertices` _array :`Triangles` (`|MakeArray` 0 2 1 2 0 3) :`UV0` (`|MakeArray` (0.0 0.0) (1.0 0.0) (1.0 1.0) (0.0 1.0) :!type "Vector2D Structure") :`VertexColors` (`|MakeArray` _trailcolor _trailcolor _trailcolor _trailcolor) :`bCreateCollision` true)
  (bind _returnvalue_3 (`PrimitiveComponent.CreateDynamicMaterialInstance` (`self.TronProceduralMesh`) 0 "/Game/Materials/M_ProceduralMesh.M_ProceduralMesh" "None"))
  (set `self.ProceduralMeshDMI` _returnvalue_3))

(fn `GetReferences`
  (returns (Success :type Boolean))
  (locals (L_Success :type Boolean :default false))
  (bind _success (`parent.GetReferences`))
  (set `local.L_Success` _success)
  (`|ExecutionSequence`
    (:`then_0`
      (bind _asbp_tron_cycle (cast `/Game/Blueprints/BP_TronCycle` (`self.GetOwner`)))
      (set `self.OwnerCycle` _asbp_tron_cycle))
    (:`then_1`
      (return false))))

(fn `UserConstructionScript`)