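; Game instance for the Tron game that handles hosting and joining multiplayer games on request.
; Direct connection requests join a host by IP through an "open" console command run on the first player controller.
; Session requests create a non-LAN session with one fewer public connection than the player count, then open GameMap as a listen server on success.
; Connection attempts and session results are shown as on-screen debug prints.
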(event `DirectConnectionRequest`
  (params (IP :type String))
  (`KismetSystemLibrary.PrintString` (`KismetStringLibrary.Concat_StrStr` "TRY TO CONNECT, IP:  " IP) true true (struct :`R` 1.0 :`B` 0.906257 :`A` 1.0) 44.0)
  (`KismetSystemLibrary.ExecuteConsoleCommand` (`KismetStringLibrary.Concat_StrStr` "open" " " IP) (`GameplayStatics.GetPlayerController` 0)))

(event `CreateSessionRequest`
  (params (PlayersNum :type Integer))
  (`CreateSessionCallbackProxy.CreateSession` (`GameplayStatics.GetPlayerController` 0) (- PlayersNum 1)
    (:`OnSuccess`
      (`GameplayStatics.OpenLevel` "GameMap" false "listen")
      (`KismetSystemLibrary.PrintString` "SESSION CREATION SUCCESS" true true (struct :`R` 1.0 :`B` 0.906257 :`A` 1.0) 44.0))
    (:`OnFailure`
      (`KismetSystemLibrary.PrintString` "SESSION CREATION FAILED" true true (struct :`R` 1.0 :`G` 0.131925 :`A` 1.0) 44.0))))