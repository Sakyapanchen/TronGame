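; BP_TronPlayerController is the player controller for a Tron game, handling client setup and camera selection when play begins.
; On BeginPlay it caches the BP_TronGameInstance reference, hides the virtual joystick and runs a console command to show the FPS counter.
; It then switches the view to the first BP_GameCamera actor found in the level, so a level camera provides the view.
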(event `self.ReceiveBeginPlay`
  (`parent.ReceiveBeginPlay`)
  (`self.GetReferences`)
  (`self.SetVirtualJoystickVisibility` false)
  (`KismetSystemLibrary.ExecuteConsoleCommand` "STAT FPS" self)
  (bind _outactors (`GameplayStatics.GetAllActorsOfClass` "/Game/Blueprints/BP_GameCamera.BP_GameCamera_C"))
  (`self.SetViewTargetWithBlend` self (`|GetArrayItem` _outactors) 0.0 "VTBlend_Linear" 0.0 false))

(fn `GetReferences`
  (bind _asbp_tron_game_instance (cast `/Game/Blueprints/BP_TronGameInstance` (`GameplayStatics.GetGameInstance`)))
  (set `self.GameInstance` _asbp_tron_game_instance))

(fn `UserConstructionScript`)